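; BP_Turret is an automatic bubblegum turret that turns toward enemies and sprays projectiles.
; On BeginPlay it plays its start montage and starts a fast looping timer that spawns Bubblegum_Projectile from the barrel socket with random pitch and yaw spread.
; Each tick it yaws the root toward the nearest Enemy-tagged actor; firing continues regardless of whether an enemy exists.
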(event `self.ReceiveBeginPlay`
  (`KismetSystemLibrary.K2_SetTimerDelegate` (delegate `Shoot`) 0.1 true)
  (`|PlayMontage` (`self.Mesh`) "/Game/Candy/AmetrallaGoma/AME_Animation/AnimMontage_Turret.AnimMontage_Turret" 1.0 0.0 "Start"))

(event `Shoot`
  (bind _returnvalue (`SceneComponent.GetSocketTransform` (`self.Mesh`) "Jn_Barrel_Ametrallagoma" "RTS_World"))
  (`|SpawnActorFromClass` "/Game/Candy/AmetrallaGoma/Bubblegum_Projectile.Bubblegum_Projectile_C" (`KismetMathLibrary.MakeTransform` (.location _returnvalue) (`KismetMathLibrary.MakeRotator` 0.0 (+ (.pitch (.rotation _returnvalue)) (`KismetMathLibrary.RandomFloatInRange` -15.0 15.0)) (+ (.yaw (.rotation _returnvalue)) (`KismetMathLibrary.RandomFloatInRange` -15.0 15.0)))) "Undefined" "OverrideRootScale" null null))

(event `self.ReceiveTick`
  (params (DeltaSeconds :type "Float (single-precision)"))
  (bind _returnvalue (`self.K2_GetActorLocation`))
  ;[1 1 1] LookAt closest enemy
  (bind _outactors (`GameplayStatics.GetAllActorsWithTag` "Enemy" :!label _label))
  (if (`KismetArrayLibrary.Array_IsNotEmpty` _outactors)
    (bind (_returnvalue_roll _returnvalue_pitch _returnvalue_yaw) (`KismetMathLibrary.BreakRotator` (`KismetMathLibrary.FindLookAtRotation` _returnvalue (`self.K2_GetActorLocation` (`.ReturnValue` (`GameplayStatics.FindNearestActor` _returnvalue _outactors))))))
    (`SceneComponent.K2_SetWorldRotation` (`self.RootComponent`) (`KismetMathLibrary.MakeRotator` 0.0 0.0 _returnvalue_yaw) false false)))

(event `Aim`
  ;[1 1 1] LookAt closest enemy
  (goto _label))

(fn `UserConstructionScript`)