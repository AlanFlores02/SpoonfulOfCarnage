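; Base building Blueprint that validates its placement and previews whether the current spot is buildable.
; On the NewPos event, it measures the distance from itself to each actor tagged "Building".
; Any actor closer than MinDistance clears BuildReady, turns the Cylinder preview material red and stops the search.
; Otherwise BuildReady stays true and the Cylinder shows the green preview material.
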(event `NewPos`
  (bind _cylinder (`self.Cylinder`))
  (set `self.Build Ready` true)
  (bind _outactors (`GameplayStatics.GetAllActorsWithTag` "Building"))
  (for _array_element _outactors
    (if (< (`KismetMathLibrary.Vector_Distance` (`self.K2_GetActorLocation` _array_element) (`self.K2_GetActorLocation`)) (`self.MinDistance`))
      (`PrimitiveComponent.SetMaterial` _cylinder 0 "/Game/Candy/Materials/Material_PreviewRed.Material_PreviewRed")
      (set `self.Build Ready` false)
      (break)))
  (if (`self.Build Ready`)
    (`PrimitiveComponent.SetMaterial` _cylinder 0 "/Game/Candy/Materials/Material_PreviewGreen.Material_PreviewGreen")))

(fn `UserConstructionScript`)