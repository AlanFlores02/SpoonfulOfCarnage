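; BP_UnlockKey is a key actor that spins at a fixed tilt and plays a celebratory animation when picked up.
; Tick advances the yaw by RotateSpeed and, through a gate opened by Pickup, moves the key steadily upward.
; Pickup also speeds up the spin and disables collider collision, then after a delay spawns confetti and shortly afterward destroys the key.
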(event `self.ReceiveTick`
  (params (DeltaSeconds :type "Float (single-precision)"))
  (bind (_returnvalue_roll _returnvalue_pitch _returnvalue_yaw) (`KismetMathLibrary.BreakRotator` (`self.K2_GetActorRotation`)))
  (`self.K2_SetActorRotation` (`KismetMathLibrary.MakeRotator` 15.0 15.0 (+ (* DeltaSeconds (`self.Rotate Speed`)) _returnvalue_yaw)))
  (`/Engine/EditorBlueprintResources/StandardMacros.Gate` true :!label _label
    (:`Exit`
      (`self.K2_SetActorLocation` (+ (`self.K2_GetActorLocation`) (`KismetMathLibrary.MakeVector` 0.0 0.0 (* DeltaSeconds 100.0)))))))

(event `Pickup`
  (`|ExecutionSequence`
    (:`then_0`
      (set `self.Rotate Speed` 720.0)
      (`PrimitiveComponent.SetCollisionEnabled` (`self.Collider`) "NoCollision")
      (goto _label :!via `Open`))
    (:`then_1`
      (`KismetSystemLibrary.Delay` 2.0)
      (`|SpawnActorFromClass` "/Game/Candy/VFX_ConfettiBP.VFX_ConfettiBP_C" (`self.GetTransform`) "Undefined" "OverrideRootScale" null null)
      (`KismetSystemLibrary.Delay` 0.5)
      (`self.K2_DestroyActor`))))

(fn `UserConstructionScript`)