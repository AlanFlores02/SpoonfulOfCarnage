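; Barricacao_BP is a damageable barricade that visibly breaks down in stages before being destroyed.
; Incoming damage lowers Health, which is compared against the checkpoint for the current stage.
; Crossing a checkpoint swaps in that stage's skeletal mesh and animation from parallel arrays, advancing at most one stage per hit.
; The stage counter triggers actor destruction after a short delay once the final stage is reached.
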(event `self.ReceiveAnyDamage`
  (params (Damage :type "Float (single-precision)") (DamageType :type "DamageType Object Reference") (InstigatedBy :type "Controller Object Reference") (DamageCauser :type "Actor Object Reference"))
  (bind _stage (`self.Stage`))
  (bind _mesh (`self.Mesh`))
  (bind _output_get (set `self.Health` (- (`self.Health`) Damage)))
  (if (<= _output_get (`|GetArrayItem` (`self.Health Checkpoints`) _stage))
    (`SkeletalMeshComponent.SetSkeletalMeshAsset` _mesh (`|GetArrayItem` (`self.Skeletons`) _stage))
    (`SkeletalMeshComponent.SetAnimation` _mesh (`|GetArrayItem` (`self.Animations`) _stage))
    (bind _result (`/Engine/EditorBlueprintResources/StandardMacros.IncrementInt` _stage)
      (:`  `
        (if (== _result 3)
          (`KismetSystemLibrary.Delay` 0.2)
          (`self.K2_DestroyActor`))))))

(fn `UserConstructionScript`)