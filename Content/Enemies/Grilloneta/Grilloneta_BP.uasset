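; Grilloneta is an enemy pawn that walks to the base by default, diverting to attack the player or Barricacao walls it sees.
; Seek records the target type and runs AI MoveTo, enabling attack on arrival; a sighted wall becomes a locked commitment.
; A looping timer runs a hand-written "Behavior Tree" function that attacks via montage and forward box trace, and re-chases or abandons the player by distance.
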(event `self.ReceiveBeginPlay`
  ;[1 1 1] Actor References
  (bind _returnvalue (`GameplayStatics.GetActorOfClass` "/Game/Candy/CASS/Base_Blueprint.Base_Blueprint_C"))
  (bind _output_get (set `self.Base Actor` _returnvalue))
  (bind _asbp_first_person_character (cast `/Game/FirstPerson/Blueprints/BP_FirstPersonCharacter` (`GameplayStatics.GetPlayerCharacter` 0)))
  (set `self.Player Actor` _asbp_first_person_character)
  (`self.Seek` 2 null _output_get)
  (bind _returnvalue_2 (`KismetSystemLibrary.K2_SetTimer` null "Behavior Tree" 1.0 true)))

(event `Die`
  (`KismetSystemLibrary.K2_PauseTimerHandle` (stale `self.ReceiveBeginPlay` _returnvalue_2))
  (`PrimitiveComponent.SetCollisionResponseToAllChannels` (`self.CapsuleComponent`) "ECR_Ignore")
  (`ActorComponent.SetActive` (`self.CharacterMovement`) false false)
  (`self.PlayAnimMontage` "/Game/Enemies/Grilloneta/GRI_Animation/Grilloneta_AnimMontage.Grilloneta_AnimMontage" 1.0 "End")
  (`KismetSystemLibrary.Delay` 1.16)
  (`self.K2_DestroyActor`))

(event `Seek`
  (params (`Target Index` :type Integer) (`Is Wall` :type "Actor Object Reference") (`New Target` :type "Actor Object Reference"))
  ;[0.3 0.15 0.1] AI Move To
  (set `self.Target` `Target Index`)
  (set `self.Obsesion` `Is Wall`)
  (`|AIMoveTo` self (0.0 0.0 0.0) `New Target` 75.0
    (:`OnSuccess`
      (`self.Toggle Attack Status` true))))

(event `self.PawnSensing.OnSeePawn`
  (params (Pawn :type "Pawn Object Reference"))
  ;[1 1 1] Previous commitment
  (if (and (not (and (== (`self.Target`) 2) (`self.Is Attacking ?`))) (not (`KismetSystemLibrary.IsValid` (`self.Obsesion`))))
    ;[1 1 1] Go to the wall
    (if (`KismetMathLibrary.ClassIsChildOf` (`GameplayStatics.GetObjectClass` Pawn) "/Game/Candy/Barricacao/Barricacao_BP.Barricacao_BP_C")
      (`self.Seek` 3 Pawn Pawn)
      (else
        ;;[1 1 1] Go to the player
        (if (`self.IsPlayerControlled` Pawn)
          (`self.Seek` 1 null Pawn))))))

(event `CustomEvent`
  (params (Damage :type "Float (single-precision)") (DamageType :type "DamageType Object Reference") (InstigatedBy :type "Controller Object Reference") (DamageCauser :type "Actor Object Reference"))
  (bind _output_get (set `self.Health` (- (`self.Health`) Damage)))
  (if (<= _output_get 0.0)
    _))

(fn `Behavior Tree`
  (locals (`Follow Distance` :type "Float (double-precision)" :default 500.0) (Damage :type "Float (double-precision)" :default 10.0))
  (bind _returnvalue (`self.K2_GetActorLocation`))
  (bind _player_actor (`self.Player Actor`))
  (bind _base_actor (`self.Base Actor`))
  (bind _returnvalue_2 (`self.GetDistanceTo` _player_actor))
  (`|ExecutionSequence`
    (:`then_0`
      (if (`self.Is Attacking ?`)
        ;[1 0 0] Attack
        (`self.PlayAnimMontage` "/Game/Enemies/Grilloneta/GRI_Animation/Grilloneta_AnimMontage.Grilloneta_AnimMontage" 1.0 "Attack")
        (bind (_outhit _returnvalue_3) (`KismetSystemLibrary.BoxTraceSingle` :`Start` _returnvalue :`End` (+ _returnvalue (* (`self.GetActorForwardVector`) 120.0)) :`HalfSize` (20.0 20.0 20.0) :`TraceChannel` "TraceTypeQuery2" :`DrawDebugType` "ForDuration" :`TraceColor` (struct :`G` 0.1 :`B` 1.0 :`A` 1.0) :`TraceHitColor` (struct :`R` 1.0 :`A` 1.0) :`DrawTime` 0.2))
        (if _returnvalue_3
          (`GameplayStatics.ApplyDamage` (`.HitActor` (`GameplayStatics.BreakHitResult` _outhit)) (`local.Damage`)))))
    (:`then_1`
      (`/Engine/EditorBlueprintResources/StandardMacros.CompareInt` (`self.Target`) 2
        (:`<`
          ;[1 1 1] Seek the player when they move
          (if (`KismetMathLibrary.BooleanNOR` (> _returnvalue_2 (`local.Follow Distance`)) (> _returnvalue_2 (`self.GetDistanceTo` _base_actor)))
            (if (and (`self.Is Attacking ?`) (> _returnvalue_2 150.0))
              (`self.Seek` 1 null _player_actor)
              (`self.Toggle Attack Status` false :!label _label))
            (else
              (`self.Seek` 2 null _base_actor) ; Stop following the player
              (goto _label))))))))

(fn `ReceiveAnyDamage`
  (params (Damage :type "Float (single-precision)") (DamageType :type "DamageType Object Reference") (InstigatedBy :type "Controller Object Reference") (DamageCauser :type "Actor Object Reference"))
  (bind _output_get (set `self.Health` (- (`self.Health`) Damage)))
  (if (<= _output_get 0.0)
    (`self.K2_DestroyActor`)
    (else
      (`self.Behavior Tree`))))

(fn `Toggle Attack Status`
  (params (`New Status` :type Boolean))
  (if (xor `New Status` (`self.Is Attacking ?`))
    (bind _output_get (set `self.Is Attacking ?` `New Status`))
    (if (not _output_get)
      (`self.PlayAnimMontage` "/Game/Enemies/Grilloneta/GRI_Animation/Grilloneta_AnimMontage.Grilloneta_AnimMontage" 1.0 "Walk"))))

(fn `UserConstructionScript`)